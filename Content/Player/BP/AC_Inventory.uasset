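; Player inventory component that stores item structs in a fixed-size array of U_Slot objects created by InitializeInventory.
; AddItem merges stackable items into matching stacks, recursing on remainders, while only non-stackable items take empty slots.
; Helpers validate items by non-empty name, test stack compatibility and query slots by index, where occupancy means the slot object exists.
; RemoveItem is an empty stub, and debug prints remain in validation.
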(fn `AddItem`
  (params (Item :type "/Game/Item/ItemStruct Structure"))
  (locals (`Local Item` :type "/Game/Item/ItemStruct Structure"))
  (bind _local_item (`local.Local Item`))
  (bind (_itemimage _itemname _itemdescription _itemweight _bstackable _itemcount) (break `/Game/Item/ItemStruct` _local_item))
  (bind _valid (`self.IsItemValid` Item))
  (if _valid
    (bind _output_get (set `local.Local Item` Item))
    (bind _valid_2 (`self.IsItemValid` _output_get))
    (if _valid_2
      (`KismetSystemLibrary.PrintString` "VALID")
      (else
        (`KismetSystemLibrary.PrintString` "NOT VALID")))
    (if (`.bStackable_15_C8D98D204D875B5A53BA42B436E0FAA1` (break `/Game/Item/ItemStruct` _output_get))
      (for _array_element (`self.SlotArray`)
        (bind _item (`/Game/Player/BP/U_Slot.Item` _array_element))
        (bind _valid_3 (`self.IsItemValid` _item))
        (bind _isstackable (`self.DoItemsStack` _item (`local.Local Item`)))
        (if (and _isstackable _valid_3)
          (bind (_itemimage_2 _itemname_2 _itemdescription_2 _itemweight_2 _bstackable_2 _itemcount_2 _maxitemcount) (break `/Game/Item/ItemStruct` _item))
          (bind _returnvalue (+ _itemcount_2 (`KismetMathLibrary.Min` (- _maxitemcount _itemcount_2) (`.itemCount_18_27533C584C1710F15835D181AC313F05` (break `/Game/Item/ItemStruct` (`local.Local Item`))))))
          (`|VariableSetRef` _itemcount_2 _returnvalue)
          (`|VariableSetRef` _itemcount _returnvalue)
          (if (> _itemcount 0)
            (`self.AddItem` _local_item))
          (return)))
      (else
        (for (_array_element_2 _array_index) (`self.SlotArray`)
          (bind _valid_4 (`self.IsItemValid` (`/Game/Player/BP/U_Slot.Item` _array_element_2)))
          (if (not _valid_4)
            (set `/Game/Player/BP/U_Slot.Item` (`local.Local Item`) _array_element_2)
            (return)))))
    (else
      (`KismetSystemLibrary.PrintString` "Not valid item!"))))

(fn `DoItemsStack`
  (params (a :type "/Game/Item/ItemStruct Structure") (b :type "/Game/Item/ItemStruct Structure"))
  (returns (IsStackable :type Boolean))
  (bind (_itemimage _itemname _itemdescription _itemweight _bstackable _itemcount) (break `/Game/Item/ItemStruct` a))
  (bind (_itemimage_2 _itemname_2 _itemdescription_2 _itemweight_2 _bstackable_2 _itemcount_2 _maxitemcount) (break `/Game/Item/ItemStruct` b))
  (return (and (`KismetStringLibrary.EqualEqual_StrStr` _itemname _itemname_2) (and _bstackable _bstackable_2) (< _itemcount _maxitemcount))))

(fn `GetItemInSlot`
  (params (`Slot Index` :type Integer))
  (returns (Item :type "/Game/Player/BP/U_Slot Object Reference"))
  (bind _output (`|GetArrayItem` (`self.SlotArray`) `Slot Index`))
  (`/Engine/EditorBlueprintResources/StandardMacros.IsValid` _output
    (:`Is Valid`
      (return _output))
    (:`Is Not Valid`
      (bind _returnvalue (`|GenericCreateObject` "/Game/Player/BP/U_Slot.U_Slot_C"))
      (return _returnvalue))))

(fn `InitializeInventory`
  (params (numberOfSlots :type Integer))
  (`KismetArrayLibrary.Array_Resize` (`self.SlotArray`) numberOfSlots)
  (for (_ _array_index) (`self.SlotArray`)
    (bind _returnvalue (`|GenericCreateObject` "/Game/Player/BP/U_Slot.U_Slot_C"))
    (`KismetArrayLibrary.Array_Set` (`self.SlotArray`) _array_index _returnvalue)))

(fn `IsItemValid`
  (params (`Item Structure` :type "/Game/Item/ItemStruct Structure"))
  (returns (Valid :type Boolean))
  (bind _returnvalue (not (`KismetStringLibrary.IsEmpty` (`.itemName_2_ECA4657143D07666B4441AB2AE8F0A01` (break `/Game/Item/ItemStruct` `Item Structure`)))))
  (if _returnvalue
    (`KismetSystemLibrary.PrintString` "Not empty!")
    (else
      (`KismetSystemLibrary.PrintString` "Empty!")))
  (return _returnvalue))

(fn `IsSlotOccupied`
  (params (`Slot Index` :type Integer))
  (returns (`Occupied?` :type Boolean))
  (bind _slotarray (`self.SlotArray`))
  (return (and (>= `Slot Index` 0) (< `Slot Index` (`KismetArrayLibrary.Array_Length` _slotarray)) (`KismetArrayLibrary.Array_IsValidIndex` _slotarray `Slot Index`) (`KismetSystemLibrary.IsValid` (`|GetArrayItem` _slotarray `Slot Index`)))))

(fn `RemoveItem`
  (params (Item :type "/Game/Item/ItemStruct Structure")))